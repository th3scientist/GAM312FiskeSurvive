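; Player character Blueprint that creates the player and objective HUD widgets on BeginPlay and adds them to the viewport.
; The CraftMenu input uses a FlipFlop to create or remove the crafting widget, switching mouse cursor and input mode to match.
; A debug event prints Health, Hunger and Stamina, but the looping timer meant to drive it is disconnected.
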(event Custom|ConsoleShowStats
  (Development|PrintString (Utilities|String|Append "Health: " (Utilities|String|ToString(Float) (Variables|Default|GetHealth)) " 
Hunger: " (Utilities|String|ToString(Float) (Variables|Default|GetHunger)) " 
Stamina: " (Utilities|String|ToString(Float) (Variables|Default|GetStamina)))))

(event Custom|CraftingMenuToggle
  (bind _returnvalue (Game|GetPlayerController 0))
  (Utilities|FlowControl|FlipFlop
    (:A
      (bind _returnvalue_2 (UserInterface|CreateWidget "/Game/Widgets/Crafting_Widget.Crafting_Widget_C"))
      (UserInterface|Viewport|AddtoViewport _returnvalue_2 0)
      (Variables|/Script/Engine.PlayerController|SetbShowMouseCursor _returnvalue true)
      (Input|SetInputModeGameandUI _returnvalue _returnvalue_2 "DoNotLock" true false))
    (:B
      (Widget|RemovefromParent _returnvalue_2)
      (Variables|/Script/Engine.PlayerController|SetbShowMouseCursor _returnvalue false)
      (Input|SetInputModeGameOnly _returnvalue false)
      (Class|WidgetBlueprintLibrary|SetFocustoGameViewport))))

(event EventBeginPlay
  (bind _returnvalue (UserInterface|CreateWidget "/Game/Widgets/Player_WidgetBP.Player_WidgetBP_C"))
  (bind _output_get (Variables|Default|SetplayerUI _returnvalue))
  (UserInterface|Viewport|AddtoViewport _output_get 0)
  (bind _returnvalue_2 (UserInterface|CreateWidget "/Game/Widgets/Objective_WidgetBP.Objective_WidgetBP_C"))
  (bind _output_get_2 (Variables|Default|SetobjWidget _returnvalue_2))
  (UserInterface|Viewport|AddtoViewport _output_get_2 0))

(event Input|ActionEvents|InputActionCraftMenu
  (params (Key :type Key%20Structure :default "None"))
  (:Pressed
    (CallFunction|CraftingMenuToggle)))

(fn ConstructionScript)